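; Starry skybox Blueprint that slowly and endlessly shifts emissive intensity back and forth between two parameters in the StarrySky1Param Material Parameter Collection.
; From BeginPlay, it raises EmissiveAlpha1 while lowering EmissiveAlpha2 in small steps, then reverses when the rising value reaches one.
; The cycle runs as two looping branches paced by Delay nodes instead of Tick or a Timeline.
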(event `self.ReceiveBeginPlay`
  (bind _returnvalue (`KismetMaterialLibrary.GetScalarParameterValue` "/Game/Materials/StarrySky1Param.StarrySky1Param" "EmissiveAlpha1" :!label _label))
  (if (>= _returnvalue 1.0)
    (bind _returnvalue_2 (`KismetMaterialLibrary.GetScalarParameterValue` "/Game/Materials/StarrySky1Param.StarrySky1Param" "EmissiveAlpha2" :!label _label_2))
    (if (>= _returnvalue_2 1.0)
      (goto _label)
      (else
        (`KismetMaterialLibrary.SetScalarParameterValue` "/Game/Materials/StarrySky1Param.StarrySky1Param" "EmissiveAlpha2" (+ _returnvalue_2 0.01))
        (bind _returnvalue_3 (`KismetMaterialLibrary.GetScalarParameterValue` "/Game/Materials/StarrySky1Param.StarrySky1Param" "EmissiveAlpha1"))
        (`KismetMaterialLibrary.SetScalarParameterValue` "/Game/Materials/StarrySky1Param.StarrySky1Param" "EmissiveAlpha1" (- _returnvalue_3 0.01))
        (`KismetSystemLibrary.Delay` 0.5)
        (goto _label_2)))
    (else
      (`KismetMaterialLibrary.SetScalarParameterValue` "/Game/Materials/StarrySky1Param.StarrySky1Param" "EmissiveAlpha1" (+ _returnvalue 0.01))
      (bind _returnvalue_4 (`KismetMaterialLibrary.GetScalarParameterValue` "/Game/Materials/StarrySky1Param.StarrySky1Param" "EmissiveAlpha2"))
      (`KismetMaterialLibrary.SetScalarParameterValue` "/Game/Materials/StarrySky1Param.StarrySky1Param" "EmissiveAlpha2" (- _returnvalue_4 0.01))
      (`KismetSystemLibrary.Delay` 0.5)
      (goto _label))))

(fn `UserConstructionScript`)