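; BP_Camellia is a camellia object the first-person player can approach, with an interaction prompt and proximity highlight.
; Overlapping PickupRadius shows MyPrompt on the player's HUD, and leaving hides it.
; HighlightEvent toggles HighlightMesh by a distance check against the player controller, driven by both Tick and its own delayed self-call.
; CamelliaDestroy only hides the main mesh, leaving the actor and its overlap logic in place.
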(event `/Game/Main/Blueprints/BP_Plank.ReceiveBeginPlay`
  (bind _asfirst_person_character (cast `/Game/Main/Blueprints/FirstPersonCharacter` (`GameplayStatics.GetPlayerCharacter` 0)))
  (set `self.playerRef` _asfirst_person_character))

(event `self.PickupRadius.OnComponentBeginOverlap`
  (params (OtherActor :type "Actor Object Reference") (OtherComp :type "PrimitiveComponent Object Reference") (OtherBodyIndex :type Integer) (bFromSweep :type Boolean) (SweepResult :type "HitResult Structure (by ref)"))
  (if (`KismetMathLibrary.ClassIsChildOf` (`GameplayStatics.GetObjectClass` OtherActor) "/Game/Main/Blueprints/FirstPersonCharacter.FirstPersonCharacter_C")
    (`Widget.SetVisibility` (`/Game/Main/Blueprints/BP_HUD.InteractionPrompt` (`/Game/Main/Blueprints/FirstPersonCharacter.hudRef` (`self.playerRef`))) "Visible")
    (`TextBlock.SetText` (`/Game/Main/Blueprints/BP_HUD.InteractionPrompt` (`/Game/Main/Blueprints/FirstPersonCharacter.hudRef` (`self.playerRef`))) (`self.myPrompt`))))

(event `self.PickupRadius.OnComponentEndOverlap`
  (params (OtherActor :type "Actor Object Reference") (OtherComp :type "PrimitiveComponent Object Reference") (OtherBodyIndex :type Integer))
  (if (`KismetMathLibrary.ClassIsChildOf` (`GameplayStatics.GetObjectClass` OtherActor) "/Game/Main/Blueprints/FirstPersonCharacter.FirstPersonCharacter_C")
    (`Widget.SetVisibility` (`/Game/Main/Blueprints/BP_HUD.InteractionPrompt` (`/Game/Main/Blueprints/FirstPersonCharacter.hudRef` (`self.playerRef`))) "Hidden")))

(event `CamelliaDestroy`
  (`SceneComponent.SetVisibility` (`self.Mesh`) false false))

(event `self.ReceiveTick`
  (params (DeltaSeconds :type "Float (single-precision)"))
  (`self.Highlight Event`))

(event `Highlight Event`
  (`/Engine/EditorBlueprintResources/StandardMacros.CompareFloat` (`self.GetDistanceTo` (`GameplayStatics.GetPlayerController` 0)) 300.0
    (:`>`
      (`SceneComponent.SetVisibility` (`self.HighlightMesh`) false false))
    (:`<`
      (`SceneComponent.SetVisibility` (`self.HighlightMesh`) true false)))
  (`KismetSystemLibrary.Delay` 0.1)
  (`self.Highlight Event`))

(fn `UserConstructionScript`)