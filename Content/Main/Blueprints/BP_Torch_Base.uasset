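; Base torch Blueprint with two flipbook flame sprites and a flickering light.
; On BeginPlay, IsBlue swaps in blue flames and light color, while IsDisabled hides the flames and light.
; Tick randomizes light intensity through a DoOnce reset after a short Delay, only while IsDisabled is false.
; EnableLight shows the flames and light again but leaves IsDisabled unchanged, so a disabled torch stays without flicker.
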(event `self.ReceiveBeginPlay`
  ;[1 1 1] Sets the light and flames to use the blue version
  (if (`self.isBlue`)
    (`PaperFlipbookComponent.SetFlipbook` (`self.Flame1`) "/Game/Main/Textures/Sprites/Blue_Fire_Sprite_Anim.Blue_Fire_Sprite_Anim")
    (`PaperFlipbookComponent.SetFlipbook` (`self.Flame2`) "/Game/Main/Textures/Sprites/Blue_Fire_Sprite_Anim.Blue_Fire_Sprite_Anim")
    (`LightComponent.SetLightColor` (`self.FlameLight`) (struct :`R` 0.0988 :`G` 0.139348 :`B` 0.52 :`A` 1.0) true))
  (if (`self.isDisabled`)
    (`SceneComponent.SetVisibility` (`self.Flame1`) false false)
    (`SceneComponent.SetVisibility` (`self.Flame2`) false false)
    (`SceneComponent.SetVisibility` (`self.FlameLight`) false false)))

(event `self.ReceiveActorBeginOverlap`
  (params (OtherActor :type "Actor Object Reference")))

(event `self.ReceiveTick`
  (params (DeltaSeconds :type "Float (single-precision)"))
  (if (not (`self.isDisabled`))
    (`/Engine/EditorBlueprintResources/StandardMacros.DoOnce` false :!label _label
      (:`Completed`
        (`LightComponent.SetIntensity` (`self.FlameLight`) (`KismetMathLibrary.RandomFloatInRange` 6000.0 15000.0))
        (`KismetSystemLibrary.Delay` 0.1)
        (goto _label :!via `Reset`)))))

(event `Enable Light`
  (`SceneComponent.SetVisibility` (`self.Flame1`) true false)
  (`SceneComponent.SetVisibility` (`self.Flame2`) true false)
  (`SceneComponent.SetVisibility` (`self.FlameLight`) true false))

(fn `UserConstructionScript`)