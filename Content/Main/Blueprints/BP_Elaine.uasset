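; BP_Elaine is the Blueprint for the Elaine character, which plays an idle animation on its mesh.
; BeginPlay caches the player's FirstPersonCharacter, then starts the idle animation without looping.
; An unconnected graph section would smoothly rotate the actor toward the player within a set range, using the mesh's forward vector as the look-at start.
; Tick is empty, so that turning logic never runs.
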(event `self.ReceiveBeginPlay`
  (bind _asfirst_person_character (cast `/Game/Main/Blueprints/FirstPersonCharacter` (`GameplayStatics.GetPlayerCharacter` 0)))
  (set `self.CharacterRef` _asfirst_person_character)
  (`SkeletalMeshComponent.PlayAnimation` (`self.Mesh`) "/Game/Main/Animations/Elaine_Idle.Elaine_Idle" false))

(event `self.ReceiveTick`
  (params (DeltaSeconds :type "Float (single-precision)")))

(fn `UserConstructionScript`)