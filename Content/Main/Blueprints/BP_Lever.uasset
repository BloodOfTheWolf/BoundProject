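; Interactable lever that opens tagged hidden doors or the Undercroft gate, or serves as the pulley lever that triggers Davian's dialogue.
; Overlap shows HUD prompts and enables the E interaction, which branches on MyFunction.
; Missing-handle levers first require the Lever item to be placed.
; Delay loops animate handle rotation, while a self-calling 0.1-second update, started once from Tick, toggles the proximity highlight.
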(event `self.ReceiveActorBeginOverlap`
  (params (OtherActor :type "Actor Object Reference"))
  (if (`self.handleMissing`)
    ;[1 1 1] Display option to insert lever if the player has lever handle
    (if (`KismetMathLibrary.ClassIsChildOf` (`GameplayStatics.GetObjectClass` OtherActor) "/Game/Main/Blueprints/FirstPersonCharacter.FirstPersonCharacter_C")
      (bind _asfirst_person_character (cast `/Game/Main/Blueprints/FirstPersonCharacter` OtherActor))
      (if (and (`self.handleMissing`) (== (`.currentItemName_15_EB53ABB645BC60F845FCBDB7F3BD05F2` (break `/Game/Main/Blueprints/ST_PlayerItemInfo` (`/Game/Main/Blueprints/FirstPersonCharacter.itemInfoStructRef` _asfirst_person_character))) "Lever"))
        (`Widget.SetVisibility` (`/Game/Main/Blueprints/BP_HUD.InteractionPrompt` (`/Game/Main/Blueprints/FirstPersonCharacter.hudRef` _asfirst_person_character)) "Visible")
        (`TextBlock.SetText` (`/Game/Main/Blueprints/BP_HUD.InteractionPrompt` (`/Game/Main/Blueprints/FirstPersonCharacter.hudRef` _asfirst_person_character)) "Press [E] To Place Lever")
        (set `self.inRange` true)))
    (else
      ;[1 1 1] Display interaction prompt if player activated
      (if (and (!= (`self.alreadyTriggered`) true) (`self.playerActivated`))
        (if (`KismetMathLibrary.ClassIsChildOf` (`GameplayStatics.GetObjectClass` OtherActor) "/Game/Main/Blueprints/FirstPersonCharacter.FirstPersonCharacter_C")
          (bind _asfirst_person_character_2 (cast `/Game/Main/Blueprints/FirstPersonCharacter` (`GameplayStatics.GetPlayerCharacter` 0)))
          (`Widget.SetVisibility` (`/Game/Main/Blueprints/BP_HUD.InteractionPrompt` (`/Game/Main/Blueprints/FirstPersonCharacter.hudRef` _asfirst_person_character_2)) "Visible")
          (`TextBlock.SetText` (`/Game/Main/Blueprints/BP_HUD.InteractionPrompt` (`/Game/Main/Blueprints/FirstPersonCharacter.hudRef` _asfirst_person_character_2)) "Press [E] To Pull Lever")
          (set `self.inRange` true))))))

(event `self.ReceiveActorEndOverlap`
  (params (OtherActor :type "Actor Object Reference"))
  (if (`self.missingLever`)
    ;[1 1 1] Hide the text
    (bind _asfirst_person_character (cast `/Game/Main/Blueprints/FirstPersonCharacter` OtherActor))
    (`Widget.SetVisibility` (`/Game/Main/Blueprints/BP_HUD.InteractionPrompt` (`/Game/Main/Blueprints/FirstPersonCharacter.hudRef` _asfirst_person_character)) "Hidden")
    (`TextBlock.SetText` (`/Game/Main/Blueprints/BP_HUD.InteractionPrompt` (`/Game/Main/Blueprints/FirstPersonCharacter.hudRef` _asfirst_person_character)) "")
    (set `self.inRange` false)
    (else
      ;[1 1 1] Display interaction prompt if player activated
      (if (and (!= (`self.alreadyTriggered`) false) (`self.playerActivated`))
        (if (`KismetMathLibrary.ClassIsChildOf` (`GameplayStatics.GetObjectClass` OtherActor) "/Game/Main/Blueprints/FirstPersonCharacter.FirstPersonCharacter_C")
          (bind _asfirst_person_character_2 (cast `/Game/Main/Blueprints/FirstPersonCharacter` (`GameplayStatics.GetPlayerCharacter` 0)))
          (`Widget.SetVisibility` (`/Game/Main/Blueprints/BP_HUD.InteractionPrompt` (`/Game/Main/Blueprints/FirstPersonCharacter.hudRef` _asfirst_person_character_2)) "Hidden")
          (`TextBlock.SetText` (`/Game/Main/Blueprints/BP_HUD.InteractionPrompt` (`/Game/Main/Blueprints/FirstPersonCharacter.hudRef` _asfirst_person_character_2)) "")
          (set `self.inRange` false))))))

(event `Custom E Event`
  (if (`self.alreadyTriggered`)
    _
    (elif (`self.inRange`)
      (if (`self.missingLever`)
        (switch `string` (`self.myFunction`)
          (:`Pulley`
            (if (`self.handleMissing`)
              (`/Game/Main/Blueprints/BP_AI_Function_Library.RetrieveAudioCue` null "/Game/Audio/SFX/A_LeverPlacement.A_LeverPlacement")
              (`SceneComponent.SetVisibility` (`self.LeverHandle`) true false)
              (bind _outactors (`GameplayStatics.GetAllActorsOfClass` "/Game/Main/Blueprints/FirstPersonCharacter.FirstPersonCharacter_C"))
              (bind _item (`KismetArrayLibrary.Array_Get` _outactors))
              (`/Game/Main/Blueprints/FirstPersonCharacter.SetItemStruct` _item null 0 null "None")
              (bind _hudref (`/Game/Main/Blueprints/FirstPersonCharacter.hudRef` _item))
              (`/Game/Main/Blueprints/BP_HUD.RefreshInfo` _hudref)
              (`Widget.SetVisibility` (`/Game/Main/Blueprints/BP_HUD.InteractionPrompt` _hudref) "Hidden")
              (`TextBlock.SetText` (`/Game/Main/Blueprints/BP_HUD.InteractionPrompt` _hudref) "")
              (set `self.handleMissing` false)
              (`/Game/Main/Blueprints/BP_HUD.TextReveal` _hudref "Davian: Hm. I probably can't pull the lever and get to the lift in time.")
              (`KismetSystemLibrary.Delay` 3.0)
              (`/Game/Main/Blueprints/BP_HUD.TextReveal` _hudref "Davian: Elaine should pull the lever for me, and I can find a way to let her in from the other side.")
              (`KismetSystemLibrary.Delay` 5.0)
              (`/Game/Main/Blueprints/BP_HUD.TextHidden` _hudref)))
          (:`OpenHiddenDoor1`
            (if (`self.handleMissing`)
              (`SceneComponent.SetVisibility` (`self.LeverHandle`) true false)
              (bind _outactors_2 (`GameplayStatics.GetAllActorsOfClass` "/Game/Main/Blueprints/FirstPersonCharacter.FirstPersonCharacter_C"))
              (bind _item_2 (`KismetArrayLibrary.Array_Get` _outactors_2))
              (`/Game/Main/Blueprints/FirstPersonCharacter.SetItemStruct` _item_2 null 0 null "None")
              (bind _hudref_2 (`/Game/Main/Blueprints/FirstPersonCharacter.hudRef` _item_2))
              (`/Game/Main/Blueprints/BP_HUD.RefreshInfo` _hudref_2)
              (`Widget.SetVisibility` (`/Game/Main/Blueprints/BP_HUD.InteractionPrompt` _hudref_2) "Visible")
              (`TextBlock.SetText` (`/Game/Main/Blueprints/BP_HUD.InteractionPrompt` _hudref_2) "Press [E] To Pull Lever")
              (set `self.handleMissing` false)
              (else
                (bind _foundsound (`/Game/Main/Blueprints/BP_AI_Function_Library.RetrieveAudioCue` null "/Game/Audio/SFX/A_LeverPull.A_LeverPull" (`self.K2_GetActorLocation`)))
                (`self.Rotate Down` _foundsound)
                (`KismetSystemLibrary.Delay` 0.2)
                (bind _outactors_3 (`GameplayStatics.GetAllActorsOfClass` "/Game/Main/Blueprints/BP_sMALL_Door.BP_Small_Door_C"))
                (for _array_element _outactors_3
                  (if (`self.ActorHasTag` _array_element "HiddenDoor1")
                    (`/Game/Main/Blueprints/BP_sMALL_Door.Open` _array_element)
                    (set `self.alreadyTriggered` true)))))))
        (else
          (switch `string` (`self.myFunction`)
            (:`UndercroftGate`
              (`/Engine/EditorBlueprintResources/StandardMacros.DoOnce` false
                (:`Completed`
                  (bind _foundsound_2 (`/Game/Main/Blueprints/BP_AI_Function_Library.RetrieveAudioCue` null "/Game/Audio/SFX/A_LeverPull.A_LeverPull" (`SceneComponent.K2_GetComponentLocation` (`self.DefaultSceneRoot`))))
                  (`self.Rotate Down` _foundsound_2)
                  (bind _outactors_4 (`GameplayStatics.GetAllActorsOfClass` "/Game/Main/Blueprints/BP_Gate.BP_Gate_C"))
                  (for _array_element_2 _outactors_4
                    (if (`self.ActorHasTag` _array_element_2 "Undercroft Gate")
                      (set `/Game/Main/Blueprints/BP_Gate.isMovingUp` true _array_element_2)
                      (`/Game/Main/Blueprints/BP_Gate.Move Up (Code Version)` _array_element_2)
                      (set `self.alreadyTriggered` true)
                      (bind _outactors_5 (`GameplayStatics.GetAllActorsOfClass` "/Game/Main/Blueprints/FirstPersonCharacter.FirstPersonCharacter_C" :!label _label))
                      (bind _hudref_3 (`/Game/Main/Blueprints/FirstPersonCharacter.hudRef` (`KismetArrayLibrary.Array_Get` _outactors_5)))
                      (`/Game/Main/Blueprints/BP_HUD.RefreshInfo` _hudref_3)
                      (`Widget.SetVisibility` (`/Game/Main/Blueprints/BP_HUD.InteractionPrompt` _hudref_3) "Hidden")
                      (`TextBlock.SetText` (`/Game/Main/Blueprints/BP_HUD.InteractionPrompt` _hudref_3) ""))))))
            (:`OpenHiddenDoor2`
              (`self.Rotate Down` 0.0)
              (`KismetSystemLibrary.Delay` 0.2)
              (bind _outactors_6 (`GameplayStatics.GetAllActorsOfClass` "/Game/Main/Blueprints/BP_sMALL_Door.BP_Small_Door_C"))
              (for _array_element_3 _outactors_6
                (if (`self.ActorHasTag` _array_element_3 "HiddenDoor2")
                  (`/Game/Main/Blueprints/BP_sMALL_Door.Open` _array_element_3)
                  (set `self.alreadyTriggered` true)
                  (goto _label))))))))))

(event `self.ReceiveBeginPlay`
  (`|ExecutionSequence`
    (:`then_0`
      ;[1 1 1] Hide Handle
      (if (`self.missingLever`)
        (set `self.handleMissing` true)
        (`SceneComponent.SetVisibility` (`self.LeverHandle`) false false)))
    (:`then_1`
      ;[1 1 1] Allow this actor to run the "E" event
      (if (`self.playerActivated`)
        (`self.EnableInput` (`GameplayStatics.GetPlayerController` 0))))))

(event `self.ReceiveTick`
  (params (DeltaSeconds :type "Float (single-precision)")))

(event `Rotate Down`
  (params (SoundDuration :type "Float (double-precision)"))
  (bind _roll (.roll (`SceneComponent.K2_GetComponentRotation` (`self.HandleRotationPoint`))))
  (set `self.RotationToAdd` (`KismetMathLibrary.MakeRotator` (* (/ SoundDuration (- 84.0 (.roll (`SceneComponent.K2_GetComponentRotation` (`self.HandleRotationPoint`))))) 1000.0)))
  ;[1 1 1] Loop Until the lever is facing down
  (if (not (and (<= _roll 92.0) (>= _roll 84.0))) :!label _label_2
    (`SceneComponent.K2_AddLocalRotation` (`self.HandleRotationPoint`) (`self.RotationToAdd`) false false)
    (`KismetSystemLibrary.Delay` 0.005)
    (goto _label_2)))

(event `self.ReceiveTick`
  (params (DeltaSeconds :type "Float (single-precision)"))
  ;[1 1 1] Control the Highlight Effect
  (`/Engine/EditorBlueprintResources/StandardMacros.DoOnce` false
    (:`Completed`
      (`self.Update Highlight Effect`))))

(event `Update Highlight Effect`
  ;[1 1 1] Control the Highlight Effect
  (`/Engine/EditorBlueprintResources/StandardMacros.CompareFloat` (`self.GetDistanceTo` (`GameplayStatics.GetPlayerCharacter` 0)) (`self.HighlightDist`)
    (:`>`
      (`SceneComponent.SetVisibility` (`self.LeverHandleHighlight`) false false))
    (:`==`
      (`SceneComponent.SetVisibility` (`self.LeverHandleHighlight`) true false :!label _label_3))
    (:`<`
      (goto _label_3)))
  (`KismetSystemLibrary.Delay` 0.1)
  (`self.Update Highlight Effect`))

(event `Rotate Up`
  (bind _roll (.roll (`SceneComponent.K2_GetComponentRotation` (`self.HandleRotationPoint`))))
  ;[1 1 1] Loop Until the lever is facing up
  (if (not (and (<= _roll 2.0) (>= _roll -2.0))) :!label _label_4
    (`SceneComponent.K2_AddLocalRotation` (`self.HandleRotationPoint`) (struct :`Roll` -2.0) false false)
    (`KismetSystemLibrary.Delay` 0.005)
    (goto _label_4)))

(fn `UserConstructionScript`)