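; BP_Tombstone is a tombstone actor that displays an inscription from its Lines array.
; The construction script records the line count and the longest line's character length.
; On BeginPlay it spawns a centered, tinted text render component per non-empty line, stacked downward with a height offset based on line count.
; That loop is bounded by longest line length rather than line count.
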(event `self.ReceiveBeginPlay`
  (for _index (range (`self.LongestLine`))
    (bind _item (`KismetArrayLibrary.Array_Get` (`self.Lines`) _index))
    (if (> (`KismetStringLibrary.Len` _item) 0)
      (bind _returnvalue (`AddComponent|Text Render Component_0` :`RelativeTransform` (`KismetMathLibrary.MakeTransform` (`KismetMathLibrary.MakeVector` 20.0 0.0 (+ (+ (* _index -25.0) (* (`self.AmountOfLines`) 5.0)) 30.0)))))
      (`TextRenderComponent.SetTextRenderColor` _returnvalue (make `Color` 51 59 68 1))
      (`TextRenderComponent.SetHorizontalAlignment` _returnvalue "EHTA_Center")
      (`TextRenderComponent.K2_SetText` _returnvalue (`KismetTextLibrary.Conv_StringToText` _item))
      (`KismetArrayLibrary.Array_Add` (`self.Text Render Components`) _returnvalue))))

(fn `UserConstructionScript`
  (bind _returnvalue (`KismetArrayLibrary.Array_Length` (`self.Lines`)))
  (set `self.AmountOfLines` _returnvalue)
  (for _index (range _returnvalue)
    (set `self.LongestLine` (`KismetMathLibrary.Max` (`KismetStringLibrary.Len` (`KismetArrayLibrary.Array_Get` (`self.Lines`) _index)) (`self.LongestLine`)))))