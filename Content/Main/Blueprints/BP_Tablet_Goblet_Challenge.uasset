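; BP_Tablet_Goblet_Challenge is a tablet actor for a goblet challenge, built around three child-actor item take volumes.
; On BeginPlay it casts each TakeVolume child to BP_ItemTakeVolume and sets its MyFunction name to GobletChallenge.
; The casts are chained, so a failed cast leaves the later volumes unassigned.
; The challenge logic itself is not in this graph, and Tick, overlap and the construction script do nothing.
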(event `self.ReceiveBeginPlay`
  (bind _asbp_item_take_volume (cast `/Game/Main/Blueprints/BP_ItemTakeVolume` (`ChildActorComponent.ChildActor` (`self.TakeVolume1`))))
  (set `/Game/Main/Blueprints/BP_ItemTakeVolume.MyFunction` "GobletChallenge" _asbp_item_take_volume)
  (bind _asbp_item_take_volume_2 (cast `/Game/Main/Blueprints/BP_ItemTakeVolume` (`ChildActorComponent.ChildActor` (`self.TakeVolume2`))))
  (set `/Game/Main/Blueprints/BP_ItemTakeVolume.MyFunction` "GobletChallenge" _asbp_item_take_volume_2)
  (bind _asbp_item_take_volume_3 (cast `/Game/Main/Blueprints/BP_ItemTakeVolume` (`ChildActorComponent.ChildActor` (`self.TakeVolume3`))))
  (set `/Game/Main/Blueprints/BP_ItemTakeVolume.MyFunction` "GobletChallenge" _asbp_item_take_volume_3))

(event `self.ReceiveActorBeginOverlap`
  (params (OtherActor :type "Actor Object Reference")))

(event `self.ReceiveTick`
  (params (DeltaSeconds :type "Float (single-precision)")))

(fn `UserConstructionScript`)