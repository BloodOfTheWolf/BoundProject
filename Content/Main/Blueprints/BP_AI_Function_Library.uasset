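; Function library with helpers for tagged-actor lookup and audio, plus the goblet challenge check that opens the dining hall door.
; CastToActorWithTag tests only the first actor found, as both branches return.
; RetrieveAudioCue plays a cue in 2D or a sound at a location, returning its duration.
; The goblet check counts filled slots per tablet, keyed by first tag, then disables slot detection once all three tables are satisfied.
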(fn CasttoActorwithTag
  (params (Actor :type Actor%20Class%20Reference) (Tag :type Name))
  (bind _outactors (Actor|GetAllActorsOfClass 0 Actor))
  (for _array_element _outactors
    (if (Actor|ActorHasTag _array_element Tag)
      (return true _array_element)
      (else
        (return false _array_element)))))

(fn RetrieveAudioCue
  (params (InputCue :type Sound%20Cue%20Object%20Reference) (InputSound :type Sound%20Wave%20Object%20Reference) (TargetLocation :type Vector))
  (if (Utilities|IsValid InputCue)
    (bind _output_get (LocalVariables|SetSoundcueRef InputCue))
    (Audio|PlaySound2D 0 InputCue)
    (LocalVariables|SetDurationRef (Variables|/Script/Engine.SoundBase|GetDuration _output_get))
    (elif (Utilities|IsValid InputSound)
      (Audio|PlaySoundatLocation 0 InputSound TargetLocation)
      (LocalVariables|SetDurationRef (Variables|/Script/Engine.SoundBase|GetDuration InputSound))))
  (return (LocalVariables|GetDurationRef)))

(fn CheckforGobletChallengeCondition
  (bind _outactors (Actor|GetAllActorsOfClass 0 "/Game/Main/Blueprints/BP_Tablet_Goblet_Challenge.BP_Tablet_Goblet_Challenge_C"))
  (for _array_element _outactors
    (LocalVariables|SetgobletSlots (Utilities|Array|MakeArray (Variables|/Game/Main/Blueprints/BP_Tablet_Goblet_Challenge.BP_Tablet_Goblet_Challenge_C|GetTakeVolume1 _array_element) (Variables|/Game/Main/Blueprints/BP_Tablet_Goblet_Challenge.BP_Tablet_Goblet_Challenge_C|GetTakeVolume2 _array_element) (Variables|/Game/Main/Blueprints/BP_Tablet_Goblet_Challenge.BP_Tablet_Goblet_Challenge_C|GetTakeVolume3 _array_element)))
    (switch name (Utilities|Array|Get(acopy) (Variables|/Script/Engine.Actor|GetTags _array_element))
      (:1
        (LocalVariables|SetgobletsRequired 1)
        (bind _array_element_2 (Utilities|Array|ForEachLoopwithBreak (LocalVariables|GetgobletSlots))
          (:LoopBody
            (bind _asbp_item_take_volume (Utilities|Casting|CastToBP_ItemTakeVolume (Variables|/Script/Engine.ChildActorComponent|GetChildActor _array_element_2)))
            (if (Variables|/Game/Main/Blueprints/BP_ItemTakeVolume.BP_ItemTakeVolume_C|GetisFilled _asbp_item_take_volume)
              (LocalVariables|SetgobletsRequired (- (LocalVariables|GetgobletsRequired) 1))
              (CallFunction|RetrieveAudioCue 0 "/Game/Audio/SFX/A_GobletPlacement.A_GobletPlacement" (Transformation|GetActorLocation (Game|Player|GetPlayerPawn 0)))))
          (:Completed
            (if (== (LocalVariables|GetgobletsRequired) 0)
              (CallFunction|RetrieveAudioCue 0 "/Game/Audio/SFX/A_GobletPlacement.A_GobletPlacement" (Transformation|GetActorLocation (Game|Player|GetPlayerPawn 0)))
              (LocalVariables|Settable1Filled true)))))
      (:2
        (LocalVariables|SetgobletsRequired 3)
        (bind _array_element_3 (Utilities|Array|ForEachLoopwithBreak (LocalVariables|GetgobletSlots))
          (:LoopBody
            (bind _asbp_item_take_volume_2 (Utilities|Casting|CastToBP_ItemTakeVolume (Variables|/Script/Engine.ChildActorComponent|GetChildActor _array_element_3)))
            (if (Variables|/Game/Main/Blueprints/BP_ItemTakeVolume.BP_ItemTakeVolume_C|GetisFilled _asbp_item_take_volume_2)
              (LocalVariables|SetgobletsRequired (- (LocalVariables|GetgobletsRequired) 1))
              (CallFunction|RetrieveAudioCue 0 "/Game/Audio/SFX/A_GobletPlacement.A_GobletPlacement" (Transformation|GetActorLocation (Game|Player|GetPlayerPawn 0)))))
          (:Completed
            (if (== (LocalVariables|GetgobletsRequired) 0)
              (CallFunction|RetrieveAudioCue 0 "/Game/Audio/SFX/A_GobletPlacement.A_GobletPlacement" (Transformation|GetActorLocation (Game|Player|GetPlayerPawn 0)))
              (LocalVariables|Settable2Filled true)))))
      (:3
        (LocalVariables|SetgobletsRequired 2)
        (bind _array_element_4 (Utilities|Array|ForEachLoopwithBreak (LocalVariables|GetgobletSlots))
          (:LoopBody
            (bind _asbp_item_take_volume_3 (Utilities|Casting|CastToBP_ItemTakeVolume (Variables|/Script/Engine.ChildActorComponent|GetChildActor _array_element_4)))
            (if (Variables|/Game/Main/Blueprints/BP_ItemTakeVolume.BP_ItemTakeVolume_C|GetisFilled _asbp_item_take_volume_3)
              (LocalVariables|SetgobletsRequired (- (LocalVariables|GetgobletsRequired) 1))
              (CallFunction|RetrieveAudioCue 0 "/Game/Audio/SFX/A_GobletPlacement.A_GobletPlacement" (Transformation|GetActorLocation (Game|Player|GetPlayerPawn 0)))))
          (:Completed
            (if (== (LocalVariables|GetgobletsRequired) 0)
              (CallFunction|RetrieveAudioCue 0 "/Game/Audio/SFX/A_GobletPlacement.A_GobletPlacement" (Transformation|GetActorLocation (Game|Player|GetPlayerPawn 0)))
              (LocalVariables|Settable3Filled true)))))))
  (if (Math|Boolean|ANDBoolean (LocalVariables|Gettable1Filled) (LocalVariables|Gettable2Filled) (LocalVariables|Gettable3Filled))
    (bind _outactors_2 (Actor|GetAllActorsOfClass 0 "/Game/Main/Blueprints/BP_Tablet_Goblet_Challenge.BP_Tablet_Goblet_Challenge_C"))
    (for _array_element_5 _outactors_2
      (bind _output_get (LocalVariables|SetgobletSlots (Utilities|Array|MakeArray (Variables|/Game/Main/Blueprints/BP_Tablet_Goblet_Challenge.BP_Tablet_Goblet_Challenge_C|GetTakeVolume1 _array_element_5) (Variables|/Game/Main/Blueprints/BP_Tablet_Goblet_Challenge.BP_Tablet_Goblet_Challenge_C|GetTakeVolume2 _array_element_5) (Variables|/Game/Main/Blueprints/BP_Tablet_Goblet_Challenge.BP_Tablet_Goblet_Challenge_C|GetTakeVolume3 _array_element_5))))
      (for _array_element_6 _output_get
        (bind _asbp_item_take_volume_4 (Utilities|Casting|CastToBP_ItemTakeVolume (Variables|/Script/Engine.ChildActorComponent|GetChildActor _array_element_6)))
        (Collision|SetCollisionEnabled (Variables|/Game/Main/Blueprints/BP_ItemTakeVolume.BP_ItemTakeVolume_C|GetDetectionRadius _asbp_item_take_volume_4) "NoCollision")))
    (bind _outactors_3 (Actor|GetAllActorsOfClass 0 "/Game/Main/Blueprints/BP_Big_Door.BP_Big_Door_C"))
    (bind _array_element_7 (Utilities|Array|ForEachLoopwithBreak _outactors_3 :!label _label)
      (:LoopBody
        (if (Actor|ActorHasTag _array_element_7 "DiningHallDoor")
          (Utilities|FlowControl|Sequence
            (:then_0
              (goto _label Break))
            (:then_1
              (Default|Open _array_element_7))))))))