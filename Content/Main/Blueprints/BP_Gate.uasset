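; Gate actor that raises and lowers, with a raising sound and dust effects.
; MoveUp plays Matinee actors tagged GateMatinee, hides the dust owner after a delay and plays the sound slightly after starting.
; Alternative CodeVersion events step the actor's Z through short Delay loops while direction flags are set, stopping within hardcoded world-height bands.
; The code-driven raise plays the sound immediately and hides dust particles at the top.
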(event `self.ReceiveBeginPlay`)

(event `self.ReceiveActorBeginOverlap`
  (params (OtherActor :type "Actor Object Reference")))

(event `self.ReceiveTick`
  (params (DeltaSeconds :type "Float (single-precision)")))

(event `Move Up`
  (`|ExecutionSequence`
    (:`then_0`
      (bind _outactors (`GameplayStatics.GetAllActorsOfClass` "/Script/Engine.MatineeActor"))
      (for _array_element _outactors
        (if (`self.ActorHasTag` _array_element "GateMatinee")
          (`MatineeActor.Play` _array_element)
          (`KismetSystemLibrary.Delay` 3.0)
          (`SceneComponent.SetHiddenInGame` (`self.DustOwner`) true true))))
    (:`then_1`
      (`KismetSystemLibrary.Delay` 1.0)
      (`GameplayStatics.PlaySoundAtLocation` "/Game/Audio/SFX/A_GateRaising.A_GateRaising" (`SceneComponent.K2_GetComponentLocation` (`self.DefaultSceneRoot`)) :!label _label))))

(event `Move Up (Code Version)`
  (bind _z (.z (`self.K2_GetActorLocation`)))
  (`|ExecutionSequence`
    (:`then_0`
      (goto _label))
    (:`then_1`
      ;[1 1 1] Loop Gate is fully raised
      (if (`self.isMovingUp`) :!label _label_2
        (if (and (<= _z 460.0) (>= _z 440.0))
          (set `self.isMovingUp` false)
          (`SceneComponent.SetVisibility` (`self.DustParticles`) false false)
          (else
            (`self.K2_SetActorLocation` (`KismetMathLibrary.MakeVector` (.x (`self.K2_GetActorLocation`)) (.y (`self.K2_GetActorLocation`)) (+ (.z (`self.K2_GetActorLocation`)) 3.0)))
            (`KismetSystemLibrary.Delay` 0.005)
            (goto _label_2)))))))

(event `Move Down (Code Version)`
  (bind _z (.z (`self.K2_GetActorLocation`)))
  ;[1 1 1] Loop Gate is fully raised
  (if (`self.isMovingDown`) :!label _label_3
    (if (and (<= _z 60.0) (>= _z 40.0))
      (set `self.isMovingDown` false)
      (else
        (`self.K2_SetActorLocation` (`KismetMathLibrary.MakeVector` (.x (`self.K2_GetActorLocation`)) (.y (`self.K2_GetActorLocation`)) (- (.z (`self.K2_GetActorLocation`)) 3.0)))
        (`KismetSystemLibrary.Delay` 0.005)
        (goto _label_3)))))

(fn `UserConstructionScript`)