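; BP_ElaineDialogueUser is an Elaine dialogue stand-in actor that fades itself out when its Decay event fires.
; Decay caches the first-person player character, then loops on a short delay, lowering MeshAlpha and writing it to the CustomAlphaFade parameter of a material parameter collection.
; Once alpha reaches zero, it tells the player to show Elaine's body via ElaineBodyVisible and destroys itself.
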(event `Decay`
  (bind _meshalpha (`self.MeshAlpha`))
  (`|ExecutionSequence`
    (:`then_0`
      (bind _asfirst_person_character (cast `/Game/Main/Blueprints/FirstPersonCharacter` (`GameplayStatics.GetPlayerCharacter` 0)))
      (set `self.Player` _asfirst_person_character))
    (:`then_1`
      (if (<= _meshalpha 0.0) :!label _label
        (`/Game/Main/Blueprints/FirstPersonCharacter.ElaineBodyVisible` (`self.Player`))
        (`self.K2_DestroyActor`)
        (else
          (`KismetMaterialLibrary.SetScalarParameterValue` "/Game/Materials/ElaineStaticMatParam.ElaineStaticMatParam" "CustomAlphaFade" _meshalpha)
          (set `self.MeshAlpha` (- (`self.MeshAlpha`) 0.01))
          (`KismetSystemLibrary.Delay` 0.01)
          (goto _label))))))

(fn `UserConstructionScript`)