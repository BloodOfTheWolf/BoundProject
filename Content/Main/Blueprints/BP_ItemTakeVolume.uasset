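; Trigger volume that takes a required amount of a named item from the player, used for the Goblet Challenge function.
; Overlap sets InRange and shows a HUD prompt, warning what is needed if the player holds no item; leaving hides it.
; Pressing E in range with enough of the item deducts it, marks the volume filled once, clears an emptied item slot and refreshes the HUD.
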(event `self.ReceiveBeginPlay`
  (`|ExecutionSequence`
    (:`then_0`
      (bind _asfirst_person_character (cast `/Game/Main/Blueprints/FirstPersonCharacter` (`GameplayStatics.GetPlayerCharacter` 0)))
      (set `self.playerCharRef` _asfirst_person_character))
    (:`then_1`
      (`self.EnableInput` (`GameplayStatics.GetPlayerController` 0)))))

(event `self.ReceiveTick`
  (params (DeltaSeconds :type "Float (single-precision)")))

(event `self.ReceiveActorBeginOverlap`
  (params (OtherActor :type "Actor Object Reference"))
  (set `self.inRange` true)
  (switch `string` (`self.MyFunction`)
    (:`GobletChallenge`
      (if (== OtherActor (`self.playerCharRef`))
        (if (== (`.currentItemName_15_EB53ABB645BC60F845FCBDB7F3BD05F2` (break `/Game/Main/Blueprints/ST_PlayerItemInfo` (`/Game/Main/Blueprints/FirstPersonCharacter.itemInfoStructRef` (`self.playerCharRef`)))) "None")
          (`TextBlock.SetText` (`/Game/Main/Blueprints/BP_HUD.InteractionPrompt` (`/Game/Main/Blueprints/FirstPersonCharacter.hudRef` (`self.playerCharRef`))) (`KismetTextLibrary.Conv_StringToText` (`KismetStringLibrary.Concat_StrStr` "You Need [" (`KismetStringLibrary.Conv_IntToString` (`self.myItemAmount`)) "] " (`KismetStringLibrary.Conv_NameToString` (`self.myItemToTake`)))))
          (`Widget.SetVisibility` (`/Game/Main/Blueprints/BP_HUD.InteractionPrompt` (`/Game/Main/Blueprints/FirstPersonCharacter.hudRef` (`self.playerCharRef`))) "Visible")
          (else
            (`TextBlock.SetText` (`/Game/Main/Blueprints/BP_HUD.InteractionPrompt` (`/Game/Main/Blueprints/FirstPersonCharacter.hudRef` (`self.playerCharRef`))) (`self.myPrompt`))
            (`Widget.SetVisibility` (`/Game/Main/Blueprints/BP_HUD.InteractionPrompt` (`/Game/Main/Blueprints/FirstPersonCharacter.hudRef` (`self.playerCharRef`))) "Visible")))))))

(event `Key|E` :consume false
  (params (Key :type "Key Structure" :default "AnyKey"))
  (bind _myitemamount (`self.myItemAmount`))
  (bind _playercharref (`self.playerCharRef`))
  (bind (_currentitem _currentitemquantity _currentitemimage _currentitemname) (break `/Game/Main/Blueprints/ST_PlayerItemInfo` (`/Game/Main/Blueprints/FirstPersonCharacter.itemInfoStructRef` (`self.playerCharRef`))))
  (bind (_currentitem_2 _currentitemquantity_2 _currentitemimage_2 _currentitemname_2) (break `/Game/Main/Blueprints/ST_PlayerItemInfo` (`/Game/Main/Blueprints/FirstPersonCharacter.itemInfoStructRef` _playercharref)))
  (:`Pressed`
    (if (`self.inRange`)
      (switch `string` (`self.MyFunction`)
        (:`GobletChallenge`
          (if (`self.isFilled`)
            _
            (elif (and (== _currentitemname (`self.myItemToTake`)) (>= _currentitemquantity _myitemamount))
              (set `/Game/Main/Blueprints/FirstPersonCharacter.itemInfoStructRef` (make `/Game/Main/Blueprints/ST_PlayerItemInfo` _currentitem_2 (- _currentitemquantity_2 _myitemamount) _currentitemimage_2 _currentitemname_2) _playercharref)
              (set `self.isFilled` true)
              (if (> (`.currentItemQuantity_9_469646D145E1C02B205065907DA4C884` (break `/Game/Main/Blueprints/ST_PlayerItemInfo` (`/Game/Main/Blueprints/FirstPersonCharacter.itemInfoStructRef` (`self.playerCharRef`)))) 0)
                (`/Game/Main/Blueprints/BP_HUD.RefreshInfo` (`/Game/Main/Blueprints/FirstPersonCharacter.hudRef` (`self.playerCharRef`)))
                (else
                  (set `/Game/Main/Blueprints/FirstPersonCharacter.itemInfoStructRef` (make `/Game/Main/Blueprints/ST_PlayerItemInfo` null) (`self.playerCharRef`))
                  (`/Game/Main/Blueprints/BP_HUD.RefreshInfo` (`/Game/Main/Blueprints/FirstPersonCharacter.hudRef` (`self.playerCharRef`))))))))))))

(event `self.ReceiveActorEndOverlap`
  (params (OtherActor :type "Actor Object Reference"))
  (set `self.inRange` false)
  (if (== OtherActor (`self.playerCharRef`))
    (`Widget.SetVisibility` (`/Game/Main/Blueprints/BP_HUD.InteractionPrompt` (`/Game/Main/Blueprints/FirstPersonCharacter.hudRef` (`self.playerCharRef`))) "Hidden")))

(fn `UserConstructionScript`)