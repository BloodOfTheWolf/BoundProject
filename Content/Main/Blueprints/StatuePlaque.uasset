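; StatuePlaque is a plaque that displays an array of text lines on its Cube mesh.
; The construction script counts the lines, records the longest line's length and caches the Cube's world scale.
; BeginPlay spawns a centered white TextRenderComponent for each non-empty line, stacking them vertically using line count, text height and sign scale.
; A font switch by line index is left disconnected, and the longest-line value goes unused here.
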(event `self.ReceiveBeginPlay`
  (bind _textheight (`self.TextHeight`))
  (for _index (range (`self.AmountOfLines`))
    (bind _item (`KismetArrayLibrary.Array_Get` (`self.Lines`) _index))
    (if (> (`KismetStringLibrary.Len` _item) 0)
      (bind _returnvalue (`AddComponent|TextRenderComponent_0` :`RelativeTransform` (`KismetMathLibrary.MakeTransform` (`KismetMathLibrary.MakeVector` 5.0 0.0 (+ (+ (* _index (* (* _textheight -30.0) (.z (`self.SignScaleVector`)))) (* (`self.AmountOfLines`) (* _textheight 5.0))) (`self.TextHeightOrientation`))) (struct) (`KismetMathLibrary.MakeVector` 1.0 (`self.TextWidth`) (`self.TextHeight`)))))
      (`TextRenderComponent.SetHorizontalAlignment` _returnvalue "EHTA_Center")
      (`TextRenderComponent.SetTextRenderColor` _returnvalue (make `Color` 255 255 255 1))
      (`TextRenderComponent.K2_SetText` _returnvalue (`KismetTextLibrary.Conv_StringToText` _item))
      (`KismetArrayLibrary.Array_Add` (`self.TextRenderComponents`) _returnvalue))))

(fn `UserConstructionScript`
  (bind _returnvalue (`KismetArrayLibrary.Array_Length` (`self.Lines`)))
  (set `self.AmountOfLines` _returnvalue)
  (for _index (range _returnvalue)
    (set `self.LongestLine` (`KismetMathLibrary.Max` (`KismetStringLibrary.Len` (`KismetArrayLibrary.Array_Get` (`self.Lines`) _index)) (`self.LongestLine`)))
    (set `self.SignScaleVector` (`SceneComponent.K2_GetComponentScale` (`self.Cube`)))))