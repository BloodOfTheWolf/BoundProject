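; Small hinged door actor that swings open and closed through its Open and Close events, with no trigger logic of its own.
; Each event steps the right pivot's world yaw one degree, waits OpenSpeed seconds, then calls itself until within tolerance of OpenToValue or CloseToValue.
; Open plays the door sound through a DoOnce that is never reset.
; Close is silent and prints the current yaw each step.
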(event `self.ReceiveActorBeginOverlap`
  (params (OtherActor :type "Actor Object Reference")))

(event `self.ReceiveTick`
  (params (DeltaSeconds :type "Float (single-precision)")))

(event `Open`
  (`|ExecutionSequence`
    (:`then_0`
      (`/Engine/EditorBlueprintResources/StandardMacros.DoOnce` false
        (:`Completed`
          (`GameplayStatics.PlaySoundAtLocation` "/Game/Audio/FinalSFX/SmallDoorCue.SmallDoorCue" (`self.K2_GetActorLocation`)))))
    (:`then_1`
      (if (not (`KismetMathLibrary.NearlyEqual_FloatFloat` (.yaw (`SceneComponent.K2_GetComponentRotation` (`self.Door_Right_Pivot`))) (`self.OpenToValue`) 2.0))
        (`SceneComponent.K2_SetWorldRotation` (`self.Door_Right_Pivot`) (`KismetMathLibrary.MakeRotator` (.roll (`SceneComponent.K2_GetComponentRotation` (`self.Door_Right_Pivot`))) (.pitch (`SceneComponent.K2_GetComponentRotation` (`self.Door_Right_Pivot`))) (- (.yaw (`SceneComponent.K2_GetComponentRotation` (`self.Door_Right_Pivot`))) 1.0)) false false)
        (`KismetSystemLibrary.Delay` (`self.OpenSpeed`))
        (`self.Open`)))))

(event `Close`
  (bind _yaw (.yaw (`SceneComponent.K2_GetComponentRotation` (`self.Door_Right_Pivot`))))
  (`KismetSystemLibrary.PrintString` (`KismetStringLibrary.Conv_DoubleToString` _yaw))
  (if (not (`KismetMathLibrary.NearlyEqual_FloatFloat` _yaw (`self.CloseToValue`) 2.0))
    (`SceneComponent.K2_SetWorldRotation` (`self.Door_Right_Pivot`) (`KismetMathLibrary.MakeRotator` (.roll (`SceneComponent.K2_GetComponentRotation` (`self.Door_Right_Pivot`))) (.pitch (`SceneComponent.K2_GetComponentRotation` (`self.Door_Right_Pivot`))) (+ (.yaw (`SceneComponent.K2_GetComponentRotation` (`self.Door_Right_Pivot`))) 1.0)) false false)
    (`KismetSystemLibrary.Delay` (`self.OpenSpeed`))
    (`self.Close`)))

(fn `UserConstructionScript`)