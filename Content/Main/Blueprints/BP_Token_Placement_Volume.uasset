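; Trigger volume where the player places one specific token (Portrait, Gemstone or Camellia) toward an endgame unlock.
; Overlap shows a HUD prompt and opens a gate for the E key, which searches token widgets for the required name.
; A match removes the token from the HUD, spawns its endgame actor and marks the volume filled.
; It then tallies filled volumes, resetting on unfilled ones, and prints a third-ending message at three.
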(event `self.ReceiveBeginPlay`)

(event `self.ReceiveTick`
  (params (DeltaSeconds :type "Float (single-precision)")))

(event `self.ReceiveBeginPlay`
  (bind _asfirst_person_character (cast `/Game/Main/Blueprints/FirstPersonCharacter` (`GameplayStatics.GetPlayerCharacter` 0)))
  (set `self.playerRef` _asfirst_person_character))

(event `self.ReceiveActorBeginOverlap`
  (params (OtherActor :type "Actor Object Reference"))
  (bind _returnvalue (`KismetMathLibrary.MakeTransform` (.location (`self.GetTransform`)) (struct :`Roll` 90.0)))
  (if (`KismetMathLibrary.ClassIsChildOf` (`GameplayStatics.GetObjectClass` OtherActor) "/Game/Main/Blueprints/FirstPersonCharacter.FirstPersonCharacter_C")
    (`Widget.SetVisibility` (`/Game/Main/Blueprints/BP_HUD.InteractionPrompt` (`/Game/Main/Blueprints/FirstPersonCharacter.hudRef` (`self.playerRef`))) "Visible")
    (`TextBlock.SetText` (`/Game/Main/Blueprints/BP_HUD.InteractionPrompt` (`/Game/Main/Blueprints/FirstPersonCharacter.hudRef` (`self.playerRef`))) (`self.myPrompt`))
    (`self.EnableInput` (`GameplayStatics.GetPlayerController` 0))
    (goto _label :!via `Open`)))

(event `self.ReceiveActorEndOverlap`
  (params (OtherActor :type "Actor Object Reference"))
  (bind _returnvalue (`KismetMathLibrary.MakeTransform` (.location (`self.GetTransform`)) (struct :`Roll` 90.0)))
  (if (`KismetMathLibrary.ClassIsChildOf` (`GameplayStatics.GetObjectClass` OtherActor) "/Game/Main/Blueprints/FirstPersonCharacter.FirstPersonCharacter_C")
    (`Widget.SetVisibility` (`/Game/Main/Blueprints/BP_HUD.InteractionPrompt` (`/Game/Main/Blueprints/FirstPersonCharacter.hudRef` (`self.playerRef`))) "Hidden")
    (`|ExecutionSequence`
      (:`then_1`
        (`self.DisableInput` (`GameplayStatics.GetPlayerController` 0))
        (goto _label :!via `Close`)))))

(event `Key|E` :consume false
  (params (Key :type "Key Structure" :default "AnyKey"))
  (bind _returnvalue (`KismetMathLibrary.MakeTransform` (.location (`self.GetTransform`)) (struct :`Roll` 90.0)))
  (:`Pressed`
    (`/Engine/EditorBlueprintResources/StandardMacros.Gate` true :!label _label
      (:`Exit`
        (bind _foundwidgets (`WidgetBlueprintLibrary.GetAllWidgetsOfClass` "/Game/Main/Blueprints/BP_Token_Widget.BP_Token_Widget_C"))
        (for _array_element _foundwidgets
          (bind _asbp_token_widget (cast `/Game/Main/Blueprints/BP_Token_Widget` _array_element))
          (if (`KismetTextLibrary.EqualEqual_TextText` (`TextBlock.GetText` (`/Game/Main/Blueprints/BP_Token_Widget.TokenName` _asbp_token_widget)) (`self.myTokenToTake`))
            (switch `string` (`KismetTextLibrary.Conv_TextToString` (`self.myTokenToTake`))
              (:`Portrait`
                (bind _foundwidgets_2 (`WidgetBlueprintLibrary.GetAllWidgetsOfClass` "/Game/Main/Blueprints/BP_HUD.BP_HUD_C"))
                (bind _asbp_hud (cast `/Game/Main/Blueprints/BP_HUD` (`KismetArrayLibrary.Array_Get` _foundwidgets_2)))
                (bind _tokendisplayarray (`/Game/Main/Blueprints/BP_HUD.tokenDisplayArray` _asbp_hud))
                (for (_array_element_2 _array_index) _tokendisplayarray
                  (bind _asbp_token_widget_2 (cast `/Game/Main/Blueprints/BP_Token_Widget` _array_element_2))
                  (if (`KismetTextLibrary.EqualEqual_TextText` (`TextBlock.GetText` (`/Game/Main/Blueprints/BP_Token_Widget.TokenName` _asbp_token_widget_2)) (`self.myTokenToTake`))
                    (`KismetArrayLibrary.Array_Remove` _tokendisplayarray _array_index)
                    (`Widget.RemoveFromParent` _array_element_2)
                    (`/Game/Main/Blueprints/BP_HUD.RefreshTokenLocations` _asbp_hud)
                    (`|SpawnActorFromClass` "/Game/Main/Blueprints/BP_EndGame_Portrait.BP_EndGame_Portrait_C" _returnvalue "AlwaysSpawn" "OverrideRootScale")
                    (set `self.isFilled` true :!label _label_2)
                    (`ActorComponent.K2_DestroyComponent` (`self.Highlight`))
                    (bind _outactors (`GameplayStatics.GetAllActorsOfClass` "BP_Token_Placement_Volume_C"))
                    (for _array_element_3 _outactors
                      (if (`/Game/Main/Blueprints/BP_Token_Placement_Volume.isFilled` _array_element_3)
                        (set `self.tokensPlaced` (+ (`self.tokensPlaced`) 1))
                        (else
                          (set `self.tokensPlaced` 0))))
                    (if (== (`self.tokensPlaced`) 3)
                      (`KismetSystemLibrary.PrintString` "third ending unlcoked")))))
              (:`Gemstone`
                (bind _foundwidgets_3 (`WidgetBlueprintLibrary.GetAllWidgetsOfClass` "/Game/Main/Blueprints/BP_HUD.BP_HUD_C"))
                (bind _asbp_hud_2 (cast `/Game/Main/Blueprints/BP_HUD` (`KismetArrayLibrary.Array_Get` _foundwidgets_3)))
                (bind _tokendisplayarray_2 (`/Game/Main/Blueprints/BP_HUD.tokenDisplayArray` _asbp_hud_2))
                (for (_array_element_4 _array_index_2) _tokendisplayarray_2
                  (bind _asbp_token_widget_3 (cast `/Game/Main/Blueprints/BP_Token_Widget` _array_element_4))
                  (if (`KismetTextLibrary.EqualEqual_TextText` (`TextBlock.GetText` (`/Game/Main/Blueprints/BP_Token_Widget.TokenName` _asbp_token_widget_3)) (`self.myTokenToTake`))
                    (`KismetArrayLibrary.Array_Remove` _tokendisplayarray_2 _array_index_2)
                    (`Widget.RemoveFromParent` _array_element_4)
                    (`/Game/Main/Blueprints/BP_HUD.RefreshTokenLocations` _asbp_hud_2)
                    (`|SpawnActorFromClass` "/Game/Main/Blueprints/BP_EndGame_Stone_Piece.BP_EndGame_Stone_Piece_C" _returnvalue "AlwaysSpawn" "OverrideRootScale")
                    (goto _label_2))))
              (:`Camellia`
                (bind _foundwidgets_4 (`WidgetBlueprintLibrary.GetAllWidgetsOfClass` "/Game/Main/Blueprints/BP_HUD.BP_HUD_C"))
                (bind _asbp_hud_3 (cast `/Game/Main/Blueprints/BP_HUD` (`KismetArrayLibrary.Array_Get` _foundwidgets_4)))
                (bind _tokendisplayarray_3 (`/Game/Main/Blueprints/BP_HUD.tokenDisplayArray` _asbp_hud_3))
                (for (_array_element_5 _array_index_3) _tokendisplayarray_3
                  (bind _asbp_token_widget_4 (cast `/Game/Main/Blueprints/BP_Token_Widget` _array_element_5))
                  (if (`KismetTextLibrary.EqualEqual_TextText` (`TextBlock.GetText` (`/Game/Main/Blueprints/BP_Token_Widget.TokenName` _asbp_token_widget_4)) (`self.myTokenToTake`))
                    (`KismetArrayLibrary.Array_Remove` _tokendisplayarray_3 _array_index_3)
                    (`Widget.RemoveFromParent` _array_element_5)
                    (`/Game/Main/Blueprints/BP_HUD.RefreshTokenLocations` _asbp_hud_3)
                    (`|SpawnActorFromClass` "/Game/Main/Blueprints/BP_EndGame_Camellia.BP_EndGame_Camellia_C" _returnvalue "AlwaysSpawn" "OverrideRootScale")
                    (goto _label_2)))))))))))

(fn `UserConstructionScript`)