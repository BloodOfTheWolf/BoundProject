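; BP_Big_Door is a double door with Open and Close events that swing its left and right pivots in opposite directions.
; Each call steps world yaw by one degree until within a band near ±65 or zero, so motion depends on placed orientation.
; The right pivot's branch drives the loop, re-calling the event after an OpenSpeed delay.
; Open spawns the opening sound on every step, while Close plays none.
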(event `self.ReceiveBeginPlay`)

(event `self.ReceiveActorBeginOverlap`
  (params (OtherActor :type "Actor Object Reference")))

(event `self.ReceiveTick`
  (params (DeltaSeconds :type "Float (single-precision)")))

(event `Open`
  (bind _yaw (.yaw (`SceneComponent.K2_GetComponentRotation` (`self.Door_Right_Pivot`))))
  (bind _yaw_2 (.yaw (`SceneComponent.K2_GetComponentRotation` (`self.Door_Left_Pivot`))))
  (`|ExecutionSequence`
    (:`then_0`
      (if (not (and (>= _yaw_2 -68.0) (<= _yaw_2 -62.0)))
        (`SceneComponent.K2_SetWorldRotation` (`self.Door_Left_Pivot`) (`KismetMathLibrary.MakeRotator` (.roll (`SceneComponent.K2_GetComponentRotation` (`self.Door_Left_Pivot`))) (.pitch (`SceneComponent.K2_GetComponentRotation` (`self.Door_Left_Pivot`))) (- (.yaw (`SceneComponent.K2_GetComponentRotation` (`self.Door_Left_Pivot`))) 1.0)) false false)))
    (:`then_1`
      (if (not (and (>= _yaw 62.0) (<= _yaw 68.0)))
        (`SceneComponent.K2_SetWorldRotation` (`self.Door_Right_Pivot`) (`KismetMathLibrary.MakeRotator` (.roll (`SceneComponent.K2_GetComponentRotation` (`self.Door_Right_Pivot`))) (.pitch (`SceneComponent.K2_GetComponentRotation` (`self.Door_Right_Pivot`))) (+ (.yaw (`SceneComponent.K2_GetComponentRotation` (`self.Door_Right_Pivot`))) 1.0)) false false)
        (`KismetSystemLibrary.Delay` (`self.OpenSpeed`))
        (`self.Open`)))
    (:`then_2`
      (`GameplayStatics.SpawnSoundAtLocation` "/Game/Audio/SFX/A_BigDoorOpen.A_BigDoorOpen" (`SceneComponent.K2_GetComponentLocation` (`self.DefaultSceneRoot`))))))

(event `Close`
  (bind _yaw (.yaw (`SceneComponent.K2_GetComponentRotation` (`self.Door_Left_Pivot`))))
  (bind _yaw_2 (.yaw (`SceneComponent.K2_GetComponentRotation` (`self.Door_Right_Pivot`))))
  (`|ExecutionSequence`
    (:`then_0`
      (if (not (and (>= _yaw -2.0) (<= _yaw 2.0)))
        (`SceneComponent.K2_SetWorldRotation` (`self.Door_Left_Pivot`) (`KismetMathLibrary.MakeRotator` (.roll (`SceneComponent.K2_GetComponentRotation` (`self.Door_Left_Pivot`))) (.pitch (`SceneComponent.K2_GetComponentRotation` (`self.Door_Left_Pivot`))) (+ (.yaw (`SceneComponent.K2_GetComponentRotation` (`self.Door_Left_Pivot`))) 1.0)) false false)))
    (:`then_1`
      (if (not (and (>= _yaw_2 -2.0) (<= _yaw_2 2.0)))
        (`SceneComponent.K2_SetWorldRotation` (`self.Door_Right_Pivot`) (`KismetMathLibrary.MakeRotator` (.roll (`SceneComponent.K2_GetComponentRotation` (`self.Door_Right_Pivot`))) (.pitch (`SceneComponent.K2_GetComponentRotation` (`self.Door_Right_Pivot`))) (- (.yaw (`SceneComponent.K2_GetComponentRotation` (`self.Door_Right_Pivot`))) 1.0)) false false)
        (`KismetSystemLibrary.Delay` (`self.OpenSpeed`))
        (`self.Close`)))))

(fn `UserConstructionScript`)