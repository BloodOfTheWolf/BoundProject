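; Pressure plate whose AreaUsage setting selects what it drives when the player or BP_Elaine steps on it.
; It tracks overlapping characters and plays sound cues, acting on release once the list empties.
; Grounds raises and lowers tagged undercroft gates; Gardens sets CanResetBraziers on release.
; Halls opens tagged small and big doors, but its closing logic is never called, so they stay open.
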(event `self.ReceiveBeginPlay`
  (switch `string` (`self.areaUsage`)))

(event `self.ReceiveActorBeginOverlap`
  (params (OtherActor :type "Actor Object Reference"))
  (switch `string` (`self.areaUsage`)
    (:`Caste Grounds`
      (if (`KismetMathLibrary.ClassIsChildOf` (`GameplayStatics.GetObjectClass` OtherActor) "/Game/Main/Blueprints/FirstPersonCharacter.FirstPersonCharacter_C")
        (`KismetArrayLibrary.Array_Add` (`self.currentOverlappingCharacters`) OtherActor)
        (`/Game/Main/Blueprints/BP_AI_Function_Library.RetrieveAudioCue` null "/Game/Audio/SFX/A_PressurePlateOn.A_PressurePlateOn" (`self.K2_GetActorLocation`) :!label _label)
        (`self.Open Gate`)
        (elif (`KismetMathLibrary.ClassIsChildOf` (`GameplayStatics.GetObjectClass` OtherActor) "/Game/Main/Blueprints/BP_Elaine.BP_Elaine_C")
          (`KismetArrayLibrary.Array_Add` (`self.currentOverlappingCharacters`) OtherActor)
          (goto _label))))
    (:`Garden`
      (if (`KismetMathLibrary.ClassIsChildOf` (`GameplayStatics.GetObjectClass` OtherActor) "/Game/Main/Blueprints/FirstPersonCharacter.FirstPersonCharacter_C")
        (`KismetArrayLibrary.Array_Add` (`self.currentOverlappingCharacters`) OtherActor)
        (`/Game/Main/Blueprints/BP_AI_Function_Library.RetrieveAudioCue` null "/Game/Audio/SFX/A_PressurePlateOn.A_PressurePlateOn" (`self.K2_GetActorLocation`) :!label _label_2)
        (elif (`KismetMathLibrary.ClassIsChildOf` (`GameplayStatics.GetObjectClass` OtherActor) "/Game/Main/Blueprints/BP_Elaine.BP_Elaine_C")
          (`KismetArrayLibrary.Array_Add` (`self.currentOverlappingCharacters`) OtherActor)
          (goto _label_2))))
    (:`Halls`
      (if (`KismetMathLibrary.ClassIsChildOf` (`GameplayStatics.GetObjectClass` OtherActor) "/Game/Main/Blueprints/FirstPersonCharacter.FirstPersonCharacter_C")
        (`KismetArrayLibrary.Array_Add` (`self.currentOverlappingCharacters`) OtherActor)
        (`/Game/Main/Blueprints/BP_AI_Function_Library.RetrieveAudioCue` null "/Game/Audio/SFX/A_PressurePlateOn.A_PressurePlateOn" (`self.K2_GetActorLocation`) :!label _label_3)
        (bind _outactors (`GameplayStatics.GetAllActorsOfClass` "/Game/Main/Blueprints/BP_sMALL_Door.BP_Small_Door_C"))
        (for _array_element _outactors
          (if (`self.ActorHasTag` _array_element "PressurePlateRoomDoor")
            (`/Game/Main/Blueprints/BP_sMALL_Door.Open` _array_element)
            (bind _outactors_2 (`GameplayStatics.GetAllActorsOfClass` "/Game/Main/Blueprints/BP_Big_Door.BP_Big_Door_C"))
            (for _array_element_2 _outactors_2
              (if (`self.ActorHasTag` _array_element_2 "CastleHallsInnerDoor")
                (`/Game/Main/Blueprints/BP_Big_Door.Open` _array_element_2)))))
        (elif (`KismetMathLibrary.ClassIsChildOf` (`GameplayStatics.GetObjectClass` OtherActor) "/Game/Main/Blueprints/BP_Elaine.BP_Elaine_C")
          (`KismetArrayLibrary.Array_Add` (`self.currentOverlappingCharacters`) OtherActor)
          (goto _label_3))))))

(event `self.ReceiveTick`
  (params (DeltaSeconds :type "Float (single-precision)")))

(event `self.ReceiveActorEndOverlap`
  (params (OtherActor :type "Actor Object Reference"))
  (switch `string` (`self.areaUsage`)
    (:`Caste Grounds`
      (for (_array_element _array_index) (`self.currentOverlappingCharacters`)
        (if (== _array_element OtherActor)
          (`KismetArrayLibrary.Array_Remove` (`self.currentOverlappingCharacters`) _array_index)))
      (if (== (`KismetArrayLibrary.Array_Length` (`self.currentOverlappingCharacters`)) 0)
        (`/Game/Main/Blueprints/BP_AI_Function_Library.RetrieveAudioCue` null "/Game/Audio/SFX/A_PressurePlateOff.A_PressurePlateOff" (`self.K2_GetActorLocation`))
        (`self.Close Gate`)))
    (:`Garden`
      (for (_array_element_2 _array_index_2) (`self.currentOverlappingCharacters`)
        (if (== _array_element_2 OtherActor)
          (`KismetArrayLibrary.Array_Remove` (`self.currentOverlappingCharacters`) _array_index_2)))
      (if (== (`KismetArrayLibrary.Array_Length` (`self.currentOverlappingCharacters`)) 0)
        (`/Game/Main/Blueprints/BP_AI_Function_Library.RetrieveAudioCue` null "/Game/Audio/SFX/A_PressurePlateOff.A_PressurePlateOff" (`self.K2_GetActorLocation`))
        (set `self.canResetBraziers` true)))))

(event `Open Gate`
  (bind _outactors (`GameplayStatics.GetAllActorsOfClass` "/Game/Main/Blueprints/BP_Gate.BP_Gate_C"))
  (for _array_element _outactors
    (if (`self.ActorHasTag` _array_element "Undercroft Tunnel Gate")
      (set `/Game/Main/Blueprints/BP_Gate.isMovingDown` false _array_element)
      (set `/Game/Main/Blueprints/BP_Gate.isMovingUp` true _array_element)
      (`/Game/Main/Blueprints/BP_Gate.Move Up (Code Version)` _array_element))))

(event `Close Gate`
  (bind _outactors (`GameplayStatics.GetAllActorsOfClass` "/Game/Main/Blueprints/BP_Gate.BP_Gate_C"))
  (for _array_element _outactors
    (if (`self.ActorHasTag` _array_element "Undercroft Tunnel Gate")
      (set `/Game/Main/Blueprints/BP_Gate.isMovingDown` true _array_element)
      (set `/Game/Main/Blueprints/BP_Gate.isMovingUp` false _array_element)
      (`/Game/Main/Blueprints/BP_Gate.Move Down (Code Version)` _array_element))))

(fn `UserConstructionScript`)