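; BP_Book is an interactable book actor that shows an interaction prompt on the HUD while the first-person character overlaps it.
; BeginPlay caches the player character for HUD access.
; Overlap begin and end show or hide the prompt, toggle the actor's input and open or close a Gate.
; Pressing E enters that Gate, but nothing is wired to its output yet.
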(event `self.ReceiveBeginPlay`
  (bind _asfirst_person_character (cast `/Game/Main/Blueprints/FirstPersonCharacter` (`GameplayStatics.GetPlayerCharacter` 0)))
  (set `self.playerRef` _asfirst_person_character))

(event `self.ReceiveActorBeginOverlap`
  (params (OtherActor :type "Actor Object Reference"))
  (if (`KismetMathLibrary.ClassIsChildOf` (`GameplayStatics.GetObjectClass` OtherActor) "/Game/Main/Blueprints/FirstPersonCharacter.FirstPersonCharacter_C")
    (`Widget.SetVisibility` (`/Game/Main/Blueprints/BP_HUD.InteractionPrompt` (`/Game/Main/Blueprints/FirstPersonCharacter.hudRef` (`self.playerRef`))) "Visible")
    (`TextBlock.SetText` (`/Game/Main/Blueprints/BP_HUD.InteractionPrompt` (`/Game/Main/Blueprints/FirstPersonCharacter.hudRef` (`self.playerRef`))) (`self.myPrompt`))
    (`self.EnableInput` (`GameplayStatics.GetPlayerController` 0))
    (goto _label :!via `Open`)))

(event `self.ReceiveTick`
  (params (DeltaSeconds :type "Float (single-precision)")))

(event `self.ReceiveActorEndOverlap`
  (params (OtherActor :type "Actor Object Reference"))
  (if (`KismetMathLibrary.ClassIsChildOf` (`GameplayStatics.GetObjectClass` OtherActor) "/Game/Main/Blueprints/FirstPersonCharacter.FirstPersonCharacter_C")
    (`Widget.SetVisibility` (`/Game/Main/Blueprints/BP_HUD.InteractionPrompt` (`/Game/Main/Blueprints/FirstPersonCharacter.hudRef` (`self.playerRef`))) "Hidden")
    (`self.DisableInput` (`GameplayStatics.GetPlayerController` 0))
    (goto _label :!via `Close`)))

(event `Key|E` :consume false
  (params (Key :type "Key Structure" :default "AnyKey"))
  (:`Pressed`
    (`/Engine/EditorBlueprintResources/StandardMacros.Gate` true :!label _label)))

(fn `UserConstructionScript`)